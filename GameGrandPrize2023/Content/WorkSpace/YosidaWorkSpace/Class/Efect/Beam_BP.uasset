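; Beam effect Blueprint that fires a timed, travelling beam particle from a SkeletalMesh transform via Emit.
; Tick advances the end distance up to a maximum length, then also advances the start once emit time expires.
; A Visibility line trace between both sets the beam points, clips it at blocking hits and toggles the impact particle there.
; The intended zero-length shutdown tests Abs below zero, so it never triggers.
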(event `self.ReceiveTick`
  (params (DeltaSeconds :type "Float (single-precision)"))
  (bind _beamparticle (`self.BeamParticle`))
  (bind _beamparticle_2 (`self.BeamParticle`))
  (bind _beamhitparticle (`self.BeamHitParticle`))
  (bind _returnvalue (`SceneComponent.K2_GetComponentLocation` _beamparticle_2))
  (bind _returnvalue_2 (* DeltaSeconds (`self.BeamSpeed`)))
  (bind _returnvalue_3 (`KismetMathLibrary.GetForwardVector` (`SceneComponent.K2_GetComponentRotation` _beamparticle_2)))
  (if (`ActorComponent.IsActive` (`self.BeamParticle`))
    (`|ExecutionSequence`
      (:`then_0`
        ;[1 1 1] ビーム継続時間更新
        (set `self.EmitTimer` (+ (`self.EmitTimer`) DeltaSeconds)))
      (:`then_1`
        (if (`self.EmitStop`)
          ;[1 1 1] ビーム発射停止後
          (`self.Set Emit End Distance` (+ (`self.EmitEndDistance`) _returnvalue_2))
          (`self.Set Emit Start distance` (+ (`self.EmitStartDistance`) _returnvalue_2))
          (else
            ;[1 1 1] ビーム発射中
            (set `self.EmitStop` (>= (`self.EmitTimer`) (`self.EmitStopTime`)))
            (`self.Set Emit End Distance` (+ (`self.EmitEndDistance`) _returnvalue_2)))))
      (:`then_2`
        ;[1 1 1] ビームの長さがほぼ０になったら非アクティブ化
        (if (and (`self.EmitStop`) (< (`KismetMathLibrary.Abs` (- (`self.EmitStartDistance`) (`self.EmitEndDistance`))) 0.0))
          (`ActorComponent.Deactivate` (`self.BeamParticle`))
          (`ActorComponent.Deactivate` (`self.BeamHitParticle`))))
      (:`then_3`
        ;[1 1 1] 障害物との当たり判定
        (bind _outhit (`KismetSystemLibrary.LineTraceSingle` (+ _returnvalue (* (`self.EmitStartDistance`) _returnvalue_3)) (+ _returnvalue (* (`self.EmitEndDistance`) _returnvalue_3)) "TraceTypeQuery1"))
        (bind (_bblockinghit _binitialoverlap _time _distance _location _impactpoint _normal _impactnormal _physmat _hitactor _hitcomponent _hitbonename _bonename _hititem _elementindex _faceindex _tracestart _traceend) (`GameplayStatics.BreakHitResult` _outhit))
        (`ParticleSystemComponent.SetBeamSourcePoint` _beamparticle 0 _tracestart 0)
        (if _bblockinghit
          ;[1 1 1] 障害物に当たった時
          (`ParticleSystemComponent.SetBeamTargetPoint` _beamparticle 0 _location 0)
          (`ActorComponent.Activate` _beamhitparticle false)
          (`SceneComponent.K2_SetWorldLocation` _beamhitparticle _location false false)
          (`self.Set Emit End Distance` (`KismetMathLibrary.VSize` (- _returnvalue _location)))
          (else
            ;[1 1 1] 障害物に当たらなかった時
            (`ParticleSystemComponent.SetBeamTargetPoint` _beamparticle 0 _traceend 0)
            (`ActorComponent.Deactivate` _beamhitparticle)))))))

(fn `Emit`
  (params (`Emit Time` :type "Float (double-precision)"))
  (bind _beamparticle (`self.BeamParticle`))
  ;[1 1 1] 変数初期化
  (set `self.EmitStopTime` `Emit Time`)
  (set `self.EmitTimer` 0.0)
  (set `self.EmitStartDistance` 0.0)
  (set `self.EmitEndDistance` 0.0)
  (set `self.EmitStop` false)
  (`ActorComponent.Activate` _beamparticle false)
  (`SceneComponent.K2_SetWorldTransform` _beamparticle (`SceneComponent.GetSocketTransform` (`self.SkeletalMesh`) "None" "RTS_World") false false))

(fn `Set Emit End Distance`
  (params (Distance :type "Float (double-precision)"))
  (set `self.EmitEndDistance` (`KismetMathLibrary.FMin` Distance (`self.BeamLenMax`)))
  (`self.Set Emit Start distance` (`self.EmitStartDistance`)))

(fn `Set Emit Start distance`
  (params (`emit Start Distance` :type "Float (double-precision)"))
  (set `self.EmitStartDistance` (`KismetMathLibrary.FMin` `emit Start Distance` (`self.EmitEndDistance`))))

(fn `UserConstructionScript`)