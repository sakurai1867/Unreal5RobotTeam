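; BP_Movepoint is an actor in the minimap Blueprint folder that moves back and forth along the X axis.
; Each Tick applies MoveLocation as a local offset without sweep or delta-time scaling, so speed depends on frame rate.
; When world X passes TurnTop or TurnBottom, MoveLocation is set to a fixed step pointing back toward the range.
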(event `self.ReceiveTick`
  (params (DeltaSeconds :type "Float (single-precision)"))
  (bind _returnvalue_x (`KismetMathLibrary.BreakVector` (`self.K2_GetActorLocation`)))
  (bind _returnvalue_x_2 (`KismetMathLibrary.BreakVector` (`self.K2_GetActorLocation`)))
  (`self.K2_AddActorLocalOffset` (`self.MoveLocation`))
  (if (> _returnvalue_x (`self.TurnTop`))
    (set `self.MoveLocation` (-5.0 0.0 0.0))
    (elif (< _returnvalue_x_2 (`self.TurnBottom`))
      (set `self.MoveLocation` (5.0 0.0 0.0)))))

(fn `UserConstructionScript`)