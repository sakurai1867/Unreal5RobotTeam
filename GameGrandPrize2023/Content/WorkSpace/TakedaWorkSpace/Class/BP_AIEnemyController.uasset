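; BP_AIEnemyController is an enemy AI controller that tracks whether it can perceive the player.
; On BeginPlay it runs the BT_AIEnemy behavior tree.
; Its AI Perception update handler ignores actors other than player character 0, writing the player to the TargetActor blackboard key when sensed and clearing that key when sensing fails.
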(event `self.ReceiveBeginPlay`
  ;[1 1 1] ビヘイビアーツリーと接続
  (`self.RunBehaviorTree` "/Game/WorkSpace/TakedaWorkSpace/Class/BT_AIEnemy.BT_AIEnemy"))

(event `self.AIPerception.OnTargetPerceptionUpdated`
  (params (Actor :type "Actor Object Reference") (Stimulus :type "AIStimulus Structure"))
  ;[1 1 1] プレイヤー発見したときの挙動
  (if (== Actor (`GameplayStatics.GetPlayerCharacter` 0))
    (if (`.bSuccessfullySensed` (break `AIStimulus` Stimulus))
      ;;[1 1 1] プレイヤー発見時
      (`BlackboardComponent.SetValueAsObject` (`self.Blackboard`) "TargetActor" Actor)
      (else
        ;;[1 1 1] プレイヤー未発見時
        (`BlackboardComponent.SetValueAsObject` (`self.Blackboard`) "TargetActor" null)))))

(fn `UserConstructionScript`)